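; Game mode for a wave-based first-person zombie shooter that runs the waves, score and win condition.
; Each wave drops an ammo crate at a random location and spawns zombies scaled to the wave number, switching spawn points at quarter marks.
; Each kill adds score and counts down the remaining enemies, then starts the next wave with UI, sound and a delay.
; The final wave spawns a single boss, whose death shows the win screen.
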(event `self.ReceiveBeginPlay`
  ;[1 1 1] Start Game
  (`self.StartGame`)
  (`GameplayStatics.PlaySound2D` "/Game/_Main/Widgets/Zombies_Audio.Zombies_Audio" 1.0 1.0 0.0 null null))

(event `StartGame`
  ;[1 1 1] Start Game
  (`self.SpawnZombies`))

(event `WaveStart`
  ;[1 1 1] Start Next Wave
  (`GameplayStatics.PlaySound2D` "/Game/Sounds/Call_of_Duty_Zombies_New_Round_-_Sound_Effect__HD_.Call_of_Duty_Zombies_New_Round_-_Sound_Effect__HD_" 1.0 1.0 0.0 null null)
  (bind _asbp_first_person_character (cast `/Game/_Main/Blueprints/BP_FirstPersonCharacter` (`GameplayStatics.GetPlayerCharacter` 0)))
  (`/Game/_Main/Blueprints/BP_FirstPersonCharacter.ShowWaveUI` _asbp_first_person_character (`self.CurrentWave`))
  (`KismetSystemLibrary.Delay` 5.0)
  (`self.SpawnZombies`))

(event `SpawnZombies`
  ;[1 1 1] SpawnZombies
  (`self.SpawnAmmo`)
  (if (== (`self.CurrentWave`) (`self.MaxWaves`))
    (set `self.ZombiesLeft` 1)
    (`|SpawnActorFromClass` "/Game/Boss/BossBP.BossBP_C" (`KismetMathLibrary.Conv_VectorToTransform` (`|GetArrayItem` (`self.BossLocations`) (`KismetMathLibrary.RandomInteger` 3))) "Undefined" "MultiplyWithRoot" null null)
    (else
      (bind _output_get (set `self.ZombieTotal` (* (`self.CurrentWave`) 4)))
      (set `self.ZombiesLeft` _output_get)
      (for _index (range (+ _output_get 1))
        (if (== _index (/ (`self.ZombieTotal`) 4))
          (set `self.SpawnLocation1` (`self.SpawnLocation2`)))
        (if (== (/ (* (`self.ZombieTotal`) 3) 4) _index)
          (set `self.SpawnLocation1` (`self.SpawnLocation3`)))
        (if (== (/ (`self.ZombieTotal`) 2) _index)
          (set `self.SpawnLocation1` (`self.SpawnLocation4`))
          (else
            (`|SpawnActorFromClass` "/Game/Zombie/BP_Zombie.BP_Zombie_C" (`self.SpawnLocation1`) "Undefined" "MultiplyWithRoot" null null)))))))

(event `ZombieKilled`
  ;[1 1 1] Zombie Killed
  (set `self.Score` (+ (`self.Score`) 10))
  (bind _result (`/Engine/EditorBlueprintResources/StandardMacros.DecrementInt` (`self.ZombiesLeft`))
    (:`  `
      (if (== _result 0)
        (`self.WaveIncrement`)))))

(event `WaveIncrement`
  ;[1 1 1] UpdateWave
  (if (== (`self.CurrentWave`) (`self.MaxWaves`))
    (`self.PlayerWins`)
    (else
      (`/Engine/EditorBlueprintResources/StandardMacros.IncrementInt` (`self.CurrentWave`)
        (:`  `
          (`self.WaveStart`))))))

(event `PlayerWins`
  ;[1 1 1] WinLogic
  (bind _asbp_first_person_character (cast `/Game/_Main/Blueprints/BP_FirstPersonCharacter` (`GameplayStatics.GetPlayerCharacter` 0)))
  (`/Game/_Main/Blueprints/BP_FirstPersonCharacter.ShowWinUI` _asbp_first_person_character))

(event `SpawnAmmo`
  ;[1 1 1] Spawn Ammo Crate
  (`|SpawnActorFromClass` "/Game/_Main/Blueprints/BP_AmmoPickup.BP_AmmoPickup_C" (`KismetMathLibrary.MakeTransform` (`|GetArrayItem` (`self.AmmoCrateLocations`) (`KismetMathLibrary.RandomInteger` 5))) "Undefined" "MultiplyWithRoot" null null))

(fn `UserConstructionScript`)